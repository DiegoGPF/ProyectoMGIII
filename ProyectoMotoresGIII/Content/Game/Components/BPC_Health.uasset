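; BPC_Health is a health component that stores a PointsHealth value and provides heal and damage functions.
; HealFunc adds an amount to PointsHealth, capped at MaxHP.
; Damage sets PointsHealth to the larger of zero and the incoming amount, without subtracting from current health, and returns whether the result is zero.
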(fn `Damage`
  (params (Amount :type "Float (double-precision)"))
  (returns (`isDead?` :type Boolean))
  (bind _output_get (set `self.PointsHealth` (`KismetMathLibrary.FMax` (- 0.0 0.0) Amount)))
  (return (== _output_get 0.0)))

(fn `Heal Func`
  (params (Amount :type "Float (double-precision)"))
  (set `self.PointsHealth` (`KismetMathLibrary.FMin` (+ Amount (`self.PointsHealth`)) (`self.MaxHP`))))