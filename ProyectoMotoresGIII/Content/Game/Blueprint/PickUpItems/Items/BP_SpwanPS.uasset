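; Spawner actor that places a BP_SpeedPosTUTO pickup at its own transform on BeginPlay and respawns it through Box end-overlap events.
; An end overlap while IsSpawn is set waits, clears the flag and resets a DoOnce.
; A later end overlap passes that DoOnce, waits again, then spawns a new pickup and sets IsSpawn.
; The overlapping actor is never checked.
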(event `self.ReceiveBeginPlay`
  (`|SpawnActorFromClass` "/Game/Game/Blueprint/PickUpItems/Items/Tutorial/BP_SpeedPosTUTO.BP_SpeedPosTUTO_C" (`self.GetTransform`) "Undefined" "MultiplyWithRoot" null null)
  (set `self.isSpawn?` true))

(event `self.Box.OnComponentEndOverlap`
  (params (OverlappedComponent :type "PrimitiveComponent Object Reference") (OtherActor :type "Actor Object Reference") (OtherComp :type "PrimitiveComponent Object Reference") (OtherBodyIndex :type Integer))
  (if (`self.isSpawn?`)
    (`KismetSystemLibrary.Delay` 5.0)
    (set `self.isSpawn?` false)
    (goto _label :!via `Reset`)
    (else
      (`/Engine/EditorBlueprintResources/StandardMacros.DoOnce` false :!label _label
        (:`Completed`
          (`KismetSystemLibrary.Delay` 5.0)
          (`|SpawnActorFromClass` "/Game/Game/Blueprint/PickUpItems/Items/Tutorial/BP_SpeedPosTUTO.BP_SpeedPosTUTO_C" (`self.GetTransform`) "Undefined" "MultiplyWithRoot" null null)
          (set `self.isSpawn?` true))))))

(fn `UserConstructionScript`)