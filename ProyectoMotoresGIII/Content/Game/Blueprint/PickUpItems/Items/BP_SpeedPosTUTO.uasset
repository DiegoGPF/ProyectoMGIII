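; Tutorial speed pickup that, when consumed, sends its SpeedMov value to the consuming actor via a SpeedMov message, then destroys itself.
; Two timelines hand off to each other on finish, endlessly floating the mesh up and back by setting its relative location.
; Tick spins the mesh locally, with yaw scaled by delta time and Rotation, while roll and pitch add a fixed per-frame amount.
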(event `self.ReceiveBeginPlay`
  (`parent.ReceiveBeginPlay`)
  ;[1 1 1] AnimFloating
  (bind (_direction _newtrack_0) (`Timeline|Timeline` :!label _label)
    (:`Update`
      (`SceneComponent.K2_SetRelativeLocation` (`self.Mesh`) _newtrack_0 false false))
    (:`Finished`
      (bind (_direction_2 _newtrack_0_2) (`Timeline|Timeline_0` :!via `ReverseFromEnd`)
        (:`Update`
          (`SceneComponent.K2_SetRelativeLocation` (`self.Mesh`) _newtrack_0_2 false false))
        (:`Finished`
          (goto _label :!via `PlayFromStart`))))))

(event `self.ReceiveTick`
  (params (DeltaSeconds :type "Float (single-precision)"))
  (`parent.ReceiveTick` DeltaSeconds)
  (`SceneComponent.K2_AddLocalRotation` (`self.Mesh`) (`KismetMathLibrary.MakeRotator` 1.0 1.0 (* DeltaSeconds (`self.Rotation`))) false false))

(event `self.Consume`
  (params (Actor :type "Actor Object Reference"))
  (message `/Game/Game/Blueprint/BPI_interface/BPI_Player.SpeedMov` Actor (`self.Speed Mov`))
  (`self.K2_DestroyActor`))

(fn `UserConstructionScript`
  (`parent.UserConstructionScript`))