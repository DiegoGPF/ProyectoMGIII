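; BP_SpeedPos_Fixed is a pickup item that applies a heal amount and a movement speed value to the actor that consumes it.
; Its Consume event sends Heal and SpeedMov messages to that actor using HpAmount and SpeedMov, then destroys the pickup.
; BeginPlay, overlap and Tick are disabled stubs, and the construction script only calls the parent.
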(event `self.Consume`
  (params (Actor :type "Actor Object Reference"))
  (message `/Game/Game/Blueprint/BPI_interface/BPI_Player.Heal` Actor (`self.Hp Amount`))
  (message `/Game/Game/Blueprint/BPI_interface/BPI_Player.SpeedMov` Actor (`self.SpeedMov`))
  (`self.K2_DestroyActor`))

(fn `UserConstructionScript`
  (`parent.UserConstructionScript`))