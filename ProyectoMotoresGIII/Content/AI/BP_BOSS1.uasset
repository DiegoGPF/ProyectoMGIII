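; Boss enemy character that fights the player with three melee combo patterns and an aimed projectile, driven by BT_BOSS.
; Tick feeds health, player distance and a game-instance attack flag to the Blackboard.
; Attack events pick montages by combo counter, and HitCheckNpc sphere-traces the matching bone socket to apply damage.
; Incoming damage is halved for every type, and death releases player lock-on, spawns effects and sets IsBossDead on the game instance.
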(event `Projectileattack`
  (bind _returnvalue (`self.PlayAnimMontage` "/Game/Characters/Mamado/Animaciones/Cine/ProjectileAttack.ProjectileAttack" 3.0))
  (set `self.RangeAttackLength` _returnvalue)
  (set `/Game/AI/RotatingComponent.Target` (`GameplayStatics.GetPlayerCharacter` 0) (`self.RotatingComponent`))
  (`self.FireProjectil`))

(event `FireProjectil`
  (bind _returnvalue (`SceneComponent.K2_GetComponentLocation` (`self.ProjectileSpawnPoint`)))
  (`|SpawnActorFromClass` "/Game/AI/Projectileattack/BossProjectile.BossProjectile_C" (`KismetMathLibrary.MakeTransform` _returnvalue (`KismetMathLibrary.FindLookAtRotation` _returnvalue (`self.K2_GetActorLocation` (`GameplayStatics.GetPlayerCharacter` 0)))) "Undefined" "MultiplyWithRoot" null null))

(event `self.ReceiveTick`
  (params (DeltaSeconds :type "Float (single-precision)"))
  (`BlackboardComponent.SetValueAsFloat` (`AIBlueprintHelperLibrary.GetBlackboard` null) "BossHealth" (`/Game/Game/Components/BPC_Health.PointsHealth` (`self.BPC_Health`)))
  (bind _outactors (`GameplayStatics.GetAllActorsOfClass` "/Game/Characters/Goku/BP_Goku.BP_Goku_C"))
  (`BlackboardComponent.SetValueAsFloat` (`AIBlueprintHelperLibrary.GetBlackboard` null) "PlayerDistance" (`KismetMathLibrary.Vector_Distance` (`self.K2_GetActorLocation` self) (`self.K2_GetActorLocation` (`|GetArrayItem` _outactors))))
  (bind _asbp_game_instance (cast `/Game/Game/Blueprint/Instance/BP_GameInstance` (`GameplayStatics.GetGameInstance`)))
  (`BlackboardComponent.SetValueAsBool` (`AIBlueprintHelperLibrary.GetBlackboard` null) "IsAttacking" (`/Game/Game/Blueprint/Instance/BP_GameInstance.TriggerStopFire` _asbp_game_instance)))

(event `/Game/AI/BPI_Enemy.Attack2`
  (set `self.Pattern` 1)
  (if (not (`self.Atacking`))
    (set `self.Atacking` true)
    (`|PlayMontage` (`self.Mesh`) (select `int` (`self.AttackCount`) :`0` "/Game/Characters/Mamado/Animaciones/Punch_Montage_Mamado.Punch_Montage_Mamado" :`1` "/Game/Characters/Mamado/Animaciones/Attack_Hand_PwR_Montage_Mamado.Attack_Hand_PwR_Montage_Mamado" :`2` "/Game/Characters/Mamado/Animaciones/Heabutt_Montage_Mamado.Heabutt_Montage_Mamado" :!type "AnimMontage Object Reference") 1.0 0.3
      (:`then`
        (`/Engine/EditorBlueprintResources/StandardMacros.IncrementInt` (`self.AttackCount`)))
      (:`OnCompleted`
        (set `self.AttackCount` 0 :!label _label))
      (:`OnInterrupted`
        (`KismetSystemLibrary.RetriggerableDelay` 1.0)
        (set `self.Atacking` false)
        (goto _label)))))

(event `/Game/Game/Blueprint/BPI_interface/LockOn_interface.OnSelected`
  (`SceneComponent.SetVisibility` (`self.LockOnWidget`) true false))

(event `/Game/AI/BPI_Enemy.Attack3`
  (set `self.Pattern` 2)
  (set `/Game/AI/RotatingComponent.Target` (`GameplayStatics.GetPlayerCharacter` 0) (`self.RotatingComponent`))
  (if (not (`self.Atacking`))
    (set `self.Atacking` true)
    (`|PlayMontage` (`self.Mesh`) (select `int` (`self.AttackCount`) :`0` "/Game/Characters/Mamado/Animaciones/Attack_Hand_1R_Montage_Mamado.Attack_Hand_1R_Montage_Mamado" :`1` "/Game/Characters/Mamado/Animaciones/Attack_Hand_2L_Montage_Mamado.Attack_Hand_2L_Montage_Mamado" :`2` "/Game/Characters/Mamado/Animaciones/Attack_Hand_PwR_Montage_Mamado.Attack_Hand_PwR_Montage_Mamado" :`3` "/Game/Characters/Mamado/Animaciones/InsideCrescentKick_UE_Goku_Montage_Mamado.InsideCrescentKick_UE_Goku_Montage_Mamado" :!type "AnimMontage Object Reference") 1.0 0.3
      (:`then`
        (`/Engine/EditorBlueprintResources/StandardMacros.IncrementInt` (`self.AttackCount`)))
      (:`OnCompleted`
        (set `self.AttackCount` 0 :!label _label_2))
      (:`OnInterrupted`
        (`KismetSystemLibrary.RetriggerableDelay` 1.0)
        (set `self.Atacking` false)
        (goto _label_2)))))

(event `/Game/Game/Blueprint/BPI_interface/LockOn_interface.Deselected`
  (`SceneComponent.SetVisibility` (`self.LockOnWidget`) false false))

(event `self.Attack`
  (set `self.Pattern` 0)
  (if (`self.Atacking`)
    _
    (elif true
      (set `self.Atacking` true)
      (`|PlayMontage` (`self.Mesh`) (select `int` (`self.AttackCount`) :`0` "/Game/Characters/Mamado/Animaciones/Punch_Montage_Mamado.Punch_Montage_Mamado" :`1` "/Game/Characters/Mamado/Animaciones/Knee_Montage_Mamado.Knee_Montage_Mamado" :`2` "/Game/Characters/Mamado/Animaciones/Heabutt_Montage_Mamado.Heabutt_Montage_Mamado" :!type "AnimMontage Object Reference") 1.0 0.3
        (:`then`
          (`/Engine/EditorBlueprintResources/StandardMacros.IncrementInt` (`self.AttackCount`)))
        (:`OnCompleted`
          (set `self.AttackCount` 0 :!label _label_3))
        (:`OnInterrupted`
          (`KismetSystemLibrary.RetriggerableDelay` 1.0)
          (set `self.Atacking` false)
          (goto _label_3))))))

(event `self.ReceiveBeginPlay`
  (`AIController.RunBehaviorTree` (`AIBlueprintHelperLibrary.GetAIController` self) "/Game/AI/BT_BOSS.BT_BOSS"))

(event `self.PawnSensing.OnSeePawn`
  (params (Pawn :type "Pawn Object Reference"))
  (if (== Pawn (`GameplayStatics.GetPlayerCharacter` 0))
    (`AIController.RunBehaviorTree` (`AIBlueprintHelperLibrary.GetAIController` self) "/Game/AI/BT_BOSS.BT_BOSS")
    (bind _asbp_goku (cast `/Game/Characters/Goku/BP_Goku` (`GameplayStatics.GetPlayerCharacter` 0)))
    (set `self.PlayerReference` _asbp_goku)
    (bind _asaic_boss (cast `/Game/AI/AIC_BOSS` (`self.GetController`)))
    (`Controller.Possess` _asaic_boss null)))

(event `self.HitCheckNpc`
  (`self.HitDetect`))

(event `self.ReceiveAnyDamage`
  (params (Damage :type "Float (single-precision)") (DamageType :type "DamageType Object Reference") (InstigatedBy :type "Controller Object Reference") (DamageCauser :type "Actor Object Reference"))
  (`GameplayStatics.PlaySound2D` "/Game/Sounds/CharacterSounds/hit.hit" 1.0 1.0 0.0 null null)
  (`|PlayMontage` (`self.Mesh`) "/Game/Characters/Mamado/Animaciones/ReceivePunchToTheFace_UE_Montage_Mamado.ReceivePunchToTheFace_UE_Montage_Mamado" 2.5
    (:`then`
      ;[1 1 1] Por modificar para el BOSS
      (if (== (`GameplayStatics.GetObjectClass` DamageType) "/Game/Characters/Goku/Damage/DT_Rojo.DT_Rojo_C")
        (bind _output_get (set `self.Amount` (* Damage 0.5)))
        (bind _isdead_ (`/Game/Game/Components/BPC_Health.Damage` (`self.BPC_Health`) _output_get))
        (if _isdead_
          (`self.Death`))
        (else
          (bind _output_get_2 (set `self.Amount` (* Damage 0.5)))
          (bind _isdead__2 (`/Game/Game/Components/BPC_Health.Damage` (`self.BPC_Health`) _output_get_2))
          (if _isdead__2
            (`self.Death`)))))))

(event `Death`
  (bind _targetactor (`/Game/Characters/Goku/BP_Goku.TargetActor` (`self.PlayerReference`)))
  (set `self.Is Dead?` true)
  (`/Engine/EditorBlueprintResources/StandardMacros.IsValid` _targetactor
    (:`Is Valid`
      (if (== _targetactor self)
        (`/Game/Characters/Goku/BP_Goku.DisengageLockon` (`self.PlayerReference`))
        (`GameplayStatics.SpawnEmitterAtLocation` null)
        (`NiagaraFunctionLibrary.SpawnSystemAtLocation` "/Game/Game/Particulas/NS_DeadNPC.NS_DeadNPC" (`KismetMathLibrary.MakeVector` (.x (`self.K2_GetActorLocation`)) (.y (`self.K2_GetActorLocation`)) -10.0) (struct) (`self.GetActorScale3D`))
        (bind _asbp_game_instance (cast `/Game/Game/Blueprint/Instance/BP_GameInstance` (`GameplayStatics.GetGameInstance`)))
        (set `/Game/Game/Blueprint/Instance/BP_GameInstance.IsBossDead?` true _asbp_game_instance)
        (`self.K2_DestroyActor`)))
    (:`Is Not Valid`
      (`GameplayStatics.SpawnEmitterAtLocation` null)
      (`NiagaraFunctionLibrary.SpawnSystemAtLocation` "/Game/Game/Particulas/NS_DeadNPC.NS_DeadNPC" (`KismetMathLibrary.MakeVector` (.x (`self.K2_GetActorLocation`)) (.y (`self.K2_GetActorLocation`)) -10.0) (struct) (`self.GetActorScale3D`))
      (bind _asbp_game_instance_2 (cast `/Game/Game/Blueprint/Instance/BP_GameInstance` (`GameplayStatics.GetGameInstance`)))
      (set `/Game/Game/Blueprint/Instance/BP_GameInstance.IsBossDead?` true _asbp_game_instance_2)
      (`self.K2_DestroyActor`))))

(fn `HasWeapon`
  (returns (`Has Weapon` :type Boolean))
  (return false))

(fn `HitDetect`
  (bind _returnvalue (`SceneComponent.GetSocketLocation` (`self.Mesh`) (select `int` (`self.AttackCount`) :`0` "hand_r" :`1` "hand_r" :`2` "calf_l" :`3` "head" :!type "Name")))
  (bind _returnvalue_2 (`SceneComponent.GetSocketLocation` (`self.Mesh`) (select `int` (`self.AttackCount`) :`0` "hand_r" :`1` "hand_r" :`2` "hand_r" :`3` "head" :!type "Name")))
  (bind _returnvalue_3 (`SceneComponent.GetSocketLocation` (`self.Mesh`) (select `int` (`self.AttackCount`) :`0` "hand_r" :`1` "hand_r" :`2` "hand_l" :`3` "hand_r" :`4` "foot_l" :!type "Name")))
  (switch `int` (`self.Pattern`)
    (:`0`
      ;[1 1 1] Attack1
      (bind _outhit (`KismetSystemLibrary.SphereTraceSingleForObjects` _returnvalue _returnvalue 25.0 (`|MakeArray` "ObjectTypeQuery3" :!type "EObjectTypeQuery Enum")))
      (`GameplayStatics.ApplyDamage` (`.HitActor` (`GameplayStatics.BreakHitResult` _outhit)) 9.0 (`self.GetController`) self "/Script/Engine.DamageType"))
    (:`1`
      ;[1 1 1] Attack1
      (bind _outhit_2 (`KismetSystemLibrary.SphereTraceSingleForObjects` _returnvalue_2 _returnvalue_2 25.0 (`|MakeArray` "ObjectTypeQuery3" :!type "EObjectTypeQuery Enum")))
      (`GameplayStatics.ApplyDamage` (`.HitActor` (`GameplayStatics.BreakHitResult` _outhit_2)) 9.0 (`self.GetController`) self "/Script/Engine.DamageType"))
    (:`2`
      ;[1 1 1] Attack1
      (bind _outhit_3 (`KismetSystemLibrary.SphereTraceSingleForObjects` _returnvalue_3 _returnvalue_3 25.0 (`|MakeArray` "ObjectTypeQuery3" :!type "EObjectTypeQuery Enum")))
      (`GameplayStatics.ApplyDamage` (`.HitActor` (`GameplayStatics.BreakHitResult` _outhit_3)) 9.0 (`self.GetController`) self "/Script/Engine.DamageType"))))

(fn `IsDead`
  (returns (`is Dead?` :type Boolean))
  (return (`self.Is Dead?`)))

(fn `UserConstructionScript`)