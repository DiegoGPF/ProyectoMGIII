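; Blue tutorial melee enemy NPC that holds off attacking until first damaged, which triggers brief slow motion and ends its tutorial state.
; Attack cycles punch, knee and headbutt montages via AttackCount, which also picks the socket HitDetect sphere-traces to apply damage.
; Incoming damage plays a hit reaction and feeds BPCHealth, multiplied tenfold for the DT_Azul damage type.
; Death spawns particle and Niagara disintegration effects, then destroys the actor.
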(event `self.Attack`
  (if (`self.isTuto?`)
    _
    (elif (not (`self.Atacking`))
      (set `self.Atacking` true)
      (`|PlayMontage` (`self.Mesh`) (select `int` (`self.AttackCount`) :`0` "/Game/Characters/Goku/Animations/Punch_Montage.Punch_Montage" :`1` "/Game/Characters/Goku/Animations/Knee_Montage.Knee_Montage" :`2` "/Game/Characters/Goku/Animations/Heabutt_Montage.Heabutt_Montage" :!type "AnimMontage Object Reference") 1.5
        (:`then`
          (`/Engine/EditorBlueprintResources/StandardMacros.IncrementInt` (`self.AttackCount`)
            (:`  `
              (set `self.Atacking` false))))
        (:`OnCompleted`
          (set `self.AttackCount` 0 :!label _label)
          (set `self.Atacking` false))
        (:`OnInterrupted`
          (`KismetSystemLibrary.RetriggerableDelay` 1.5)
          (set `self.Atacking` false)
          (goto _label))))))

(event `self.HitCheckNpc`
  (`self.HitDetect`))

(event `self.ReceiveAnyDamage`
  (params (Damage :type "Float (single-precision)") (DamageType :type "DamageType Object Reference") (InstigatedBy :type "Controller Object Reference") (DamageCauser :type "Actor Object Reference"))
  (if (`self.isTuto?`)
    (`GameplayStatics.SetGlobalTimeDilation` 0.03)
    (`KismetSystemLibrary.Delay` 0.2)
    (`GameplayStatics.SetGlobalTimeDilation` 1.0)
    (set `self.isTuto?` false))
  (`GameplayStatics.PlaySound2D` "/Game/Sounds/CharacterSounds/hit.hit" 1.0 1.0 0.0 null null)
  (`|PlayMontage` (`self.Mesh`) "/Game/Characters/Goku/Animations/ReceivePunchToTheFace_UE_Montage.ReceivePunchToTheFace_UE_Montage" 1.5
    (:`then`
      (if (== (`GameplayStatics.GetObjectClass` DamageType) "/Game/Characters/Goku/Damage/DT_Azul.DT_Azul_C")
        (bind _output_get (set `self.Amount` (* Damage 10.0)))
        (bind _isdead_ (`/Game/Game/Components/BPC_Health.Damage` (`self.BPC_Health`) _output_get))
        (if _isdead_
          (`self.Death`))
        (else
          (bind _output_get_2 (set `self.Amount` (* Damage 1.0)))
          (bind _isdead__2 (`/Game/Game/Components/BPC_Health.Damage` (`self.BPC_Health`) _output_get_2))
          (if _isdead__2
            (`self.Death`)))))))

(event `Death`
  (`GameplayStatics.SpawnEmitterAtLocation` null)
  ;[1 1 1] Effecto Desintegrar
  (`NiagaraFunctionLibrary.SpawnSystemAtLocation` "/Game/Game/Particulas/NS_DeadNPCBlue.NS_DeadNPCBlue" (`KismetMathLibrary.MakeVector` (.x (`self.K2_GetActorLocation`)) (.y (`self.K2_GetActorLocation`)) -10.0))
  (`self.K2_DestroyActor`))

(fn `HasWeapon`
  (returns (`Has Weapon` :type Boolean))
  (return false))

(fn `HitDetect`
  (bind _returnvalue (`SceneComponent.GetSocketLocation` (`self.Mesh`) (select `int` (`self.AttackCount`) :`0` "hand_r" :`1` "hand_r" :`2` "calf_l" :`3` "head" :!type "Name")))
  (bind _outhit (`KismetSystemLibrary.SphereTraceSingleForObjects` _returnvalue _returnvalue 25.0 (`|MakeArray` "ObjectTypeQuery3" :!type "EObjectTypeQuery Enum")))
  (`GameplayStatics.ApplyDamage` (`.HitActor` (`GameplayStatics.BreakHitResult` _outhit)) 1.0 (`self.GetController`) self "/Script/Engine.DamageType"))

(fn `UserConstructionScript`)