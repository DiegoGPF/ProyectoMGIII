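; NPC melee fighter Blueprint that attacks with punch, knee and headbutt montages and reacts to damage with a sound and hit montage.
; Attack picks a montage by AttackCount behind an Atacking guard, which clears only after an interrupted montage and retriggerable delay.
; HitCheckNpc runs HitDetect, a sphere trace at the socket matching AttackCount that damages pawns.
; HasWeapon always returns false; the zero-health destroy logic is unconnected.
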(event `/Game/AI/BPI_Enemy.Attack`
  (if (not (`self.Atacking`))
    (set `self.Atacking` true)
    (`|PlayMontage` (`self.Mesh`) (select `int` (`self.AttackCount`) :`0` "/Game/Characters/Goku/Animations/Punch_Montage.Punch_Montage" :`1` "/Game/Characters/Goku/Animations/Knee_Montage.Knee_Montage" :`2` "/Game/Characters/Goku/Animations/Heabutt_Montage.Heabutt_Montage" :!type "AnimMontage Object Reference") 1.5
      (:`then`
        (`/Engine/EditorBlueprintResources/StandardMacros.IncrementInt` (`self.AttackCount`)))
      (:`OnCompleted`
        (set `self.AttackCount` 0 :!label _label))
      (:`OnInterrupted`
        (`KismetSystemLibrary.RetriggerableDelay` 1.5)
        (set `self.Atacking` false)
        (goto _label)))))

(event `self.ReceiveAnyDamage`
  (params (Damage :type "Float (single-precision)") (DamageType :type "DamageType Object Reference") (InstigatedBy :type "Controller Object Reference") (DamageCauser :type "Actor Object Reference"))
  (`GameplayStatics.PlaySound2D` "/Game/Sounds/CharacterSounds/hit.hit" 1.0 1.0 0.0 null null)
  (`|PlayMontage` (`self.Mesh`) "/Game/Characters/Goku/Animations/ReceivePunchToTheFace_UE_Montage.ReceivePunchToTheFace_UE_Montage" 1.5))

(event `/Game/AI/BPI_Enemy.HitCheckNpc`
  (`self.HitDetect`))

(fn `HasWeapon`
  (returns (`Has Weapon` :type Boolean))
  (return false))

(fn `HitDetect`
  (bind _returnvalue (`SceneComponent.GetSocketLocation` (`self.Mesh`) (select `int` (`self.AttackCount`) :`0` "hand_r" :`1` "hand_r" :`2` "calf_l" :`3` "head" :!type "Name")))
  (bind _outhit (`KismetSystemLibrary.SphereTraceSingleForObjects` _returnvalue _returnvalue 25.0 (`|MakeArray` "ObjectTypeQuery3" :!type "EObjectTypeQuery Enum")))
  (`GameplayStatics.ApplyDamage` (`.HitActor` (`GameplayStatics.BreakHitResult` _outhit)) 1.0 (`self.GetController`) self "/Script/Engine.DamageType"))

(fn `UserConstructionScript`)